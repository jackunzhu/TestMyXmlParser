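; Test actor that exercises a custom XML parser object (MyXmlFile) by dumping a file's contents to on-screen debug text.
; On BeginPlay it constructs the parser, loads a hardcoded local UTF-8 test file and prints a failure message if loading fails.
; On success, a recursive function walks the tree from the root node, printing each node's tag and content plus every attribute's tag and value.
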(event EventBeginPlay
  (bind _returnvalue (Game|ConstructObjectfromClass "/Script/MyXmlParser.MyXmlFile" "BP_testXmlParser"))
  (bind _output_get (Variables|Default|SetmyXmlFile _returnvalue))
  (bind _returnvalue_2 (Class|MyXmlFile|LoadFile _output_get "C:\\utf8test.xml" "ConstructFromFile"))
  (if _returnvalue_2
    (bind _returnvalue_3 (Class|MyXmlFile|GetRootNode (Variables|Default|GetmyXmlFile)))
    (bind _output_get_2 (Variables|Default|SetrootNode _returnvalue_3))
    (CallFunction|PrintNodeAllInfoRecursion _output_get_2)
    (else
      (Development|PrintString "load xml failed"))))

(event Collision|EventActorBeginOverlap
  (params (OtherActor :type Actor%20Object%20Reference)))

(event EventTick
  (params (DeltaSeconds :type Float%20%28single-precision%29)))

(fn ConstructionScript)

(fn PrintNodeInfo
  (params (node :type My%20Xml%20Node%20Object%20Reference))
  (Development|PrintString (Utilities|String|Append "node tag:" (Class|MyXmlNode|GetNodeTag node)) true true "(R=0.000000,G=0.660000,B=1.000000,A=1.000000)" 2e+02)
  (Development|PrintString (Utilities|String|Append "node content:" (Class|MyXmlNode|GetNodeContent node)) true true "(R=0.000000,G=0.660000,B=1.000000,A=1.000000)" 2e+03))

(fn PrintAttributeInfo
  (params (attribute :type My%20Xml%20Attribute%20Object%20Reference))
  (Development|PrintString (Utilities|String|Append "attribute tag:" (Class|MyXmlAttribute|GetAttributeTag attribute)) true true "(R=0.000000,G=0.660000,B=1.000000,A=1.000000)" 2e+02)
  (Development|PrintString (Utilities|String|Append "attribute value:" (Class|MyXmlAttribute|GetAttributeValue attribute)) true true "(R=0.000000,G=0.660000,B=1.000000,A=1.000000)" 2e+03))

(fn PrintNodeAllInfo
  (params (node :type My%20Xml%20Node%20Object%20Reference))
  (CallFunction|PrintNodeInfo node)
  (for _array_element (Class|MyXmlNode|GetNodeAttributes node)
    (CallFunction|PrintAttributeInfo _array_element)))

(fn PrintNodeAllInfoRecursion
  (params (node :type My%20Xml%20Node%20Object%20Reference))
  (CallFunction|PrintNodeAllInfo node)
  (bind _returnvalue (Class|MyXmlNode|GetChildrenNodes node))
  (for _array_element _returnvalue
    (CallFunction|PrintNodeAllInfoRecursion _array_element)))